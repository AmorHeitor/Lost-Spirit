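; Puzzle box that the BP_Body player can pick up, carry and drop, with sound and material feedback.
; Overlapping Y_Box shows a prompt widget and opens a gate for OnBoxInteract, which attaches the box to the body's Billboard with physics and collision off.
; Release requires the body's collision check and a WorldStatic box trace to be clear, then restores physics; a blocked trace briefly changes material.
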(event `Detach`
  ;[0.3953 1 0.2782] Return box to its original location
  (bind _colliding (`/Game/Blueprints/Character/BP_Body.CheckingBox colision` (`self.BodyReference`) :!label _label))
  (if _colliding
    _
    (elif (`self.Picked`)
      (`self.CheckColision`)
      (if (`self.Overlaped`)
        ;[0.3953 1 0.2782] Changing box colour
        (`PrimitiveComponent.SetMaterial` (`self.Box`) 0 "/Game/Art/Materials/M_MovableBoxTrans1.M_MovableBoxTrans1")
        (`GameplayStatics.PlaySoundAtLocation` "/Game/Sounds/S_Negative.S_Negative" (`self.K2_GetActorLocation`) (struct) 1.0 1.0 0.0 null null null)
        (`KismetSystemLibrary.Delay` 1.0)
        (if (`self.Picked`)
          (`PrimitiveComponent.SetMaterial` (`self.Box`) 0 "/Game/Art/Materials/M_MovableBoxTrans.M_MovableBoxTrans"))
        (else
          (`self.K2_DetachFromActor` "KeepWorld")
          (`PrimitiveComponent.SetCollisionEnabled` (`self.Box`) "QueryAndPhysics")
          (`PrimitiveComponent.SetSimulatePhysics` (`self.Box`) true)
          (`PrimitiveComponent.SetMaterial` (`self.Box`) 0 "/Game/Art/Materials/M_MovableBox.M_MovableBox")
          (set `self.Picked` false)
          (`GameplayStatics.PlaySoundAtLocation` "/Game/Sounds/Box/S_BoxRelease1_Cue.S_BoxRelease1_Cue" (`self.K2_GetActorLocation`) (struct) 1.0 1.0 0.0 null null null)
          (set `self.Dropped` true))))))

(event `/Game/Blueprints/Ingredients/BP_Interface.OnBoxInteract`
  (bind _box (`self.Box`))
  ;[0.3953 1 0.2782] Opening the gate for the player
  (`/Engine/EditorBlueprintResources/StandardMacros.Gate` true :!label _label_2
    (:`Exit`
      (if (`self.Picked`)
        (goto _label)
        (else
          ;[0.3953 1 0.2782] Attaching to the actor
          (`PrimitiveComponent.SetSimulatePhysics` _box false)
          (`PrimitiveComponent.SetCollisionEnabled` _box "NoCollision")
          (`PrimitiveComponent.SetMaterial` (`self.Box`) 0 "/Game/Art/Materials/M_MovableBoxTrans.M_MovableBoxTrans")
          (set `self.Picked` true)
          (`self.K2_AttachToComponent` (`/Game/Blueprints/Character/BP_Body.Billboard` (`self.BodyReference`)) "None" "SnapToTarget" "KeepRelative" "KeepWorld")
          (`GameplayStatics.PlaySoundAtLocation` "/Game/Sounds/Box/S_DroppingBox_Cue.S_DroppingBox_Cue" (`self.K2_GetActorLocation`) (struct) 1.0 1.0 0.0 null null null))))))

(event `self.Y_Box.OnComponentBeginOverlap`
  (params (OverlappedComponent :type "PrimitiveComponent Object Reference") (OtherActor :type "Actor Object Reference") (OtherComp :type "PrimitiveComponent Object Reference") (OtherBodyIndex :type Integer) (bFromSweep :type Boolean) (SweepResult :type "HitResult Structure (by ref)"))
  ;[0.3953 1 0.2782] Opening the gate for the player
  (bind _asbp_body (cast `/Game/Blueprints/Character/BP_Body` OtherActor))
  (`PrimitiveComponent.SetSimulatePhysics` (`self.Box`) false)
  (bind _output_get (set `self.BodyReference` _asbp_body))
  (`Widget.RemoveFromParent` (`/Game/Blueprints/Character/BP_Body.CurrentWidget` _output_get))
  (bind _returnvalue (`|CreateWidget` "/Game/UI/Widgets/WI_PushPullNewBox.WI_PushPullNewBox_C"))
  (bind _output_get_2 (set `self.Widget` _returnvalue))
  (`UserWidget.AddToViewport` _output_get_2 0)
  (goto _label_2 :!via `Open`))

(event `self.Y_Box.OnComponentEndOverlap`
  (params (OverlappedComponent :type "PrimitiveComponent Object Reference") (OtherActor :type "Actor Object Reference") (OtherComp :type "PrimitiveComponent Object Reference") (OtherBodyIndex :type Integer))
  (cast `/Game/Blueprints/Character/BP_Body` OtherActor)
  (`Widget.RemoveFromParent` (`self.Widget`))
  (`PrimitiveComponent.SetSimulatePhysics` (`self.Box`) true))

(event `self.Box.OnComponentHit`
  (params (HitComponent :type "PrimitiveComponent Object Reference") (OtherActor :type "Actor Object Reference") (OtherComp :type "PrimitiveComponent Object Reference") (NormalImpulse :type "Vector Structure") (Hit :type "HitResult Structure (by ref)"))
  ;[0.3953 1 0.2782] Reseting the physics
  (`|ExecutionSequence`
    (:`then_0`
      (if (`SceneComponent.IsAnySimulatingPhysics` (`self.Box`))
        (`PrimitiveComponent.SetSimulatePhysics` (`self.Box`) true)
        (if (`self.Dropped`)
          (`GameplayStatics.PlaySoundAtLocation` "/Game/Sounds/Box/S_RandomDrop.S_RandomDrop" (`self.K2_GetActorLocation`) (struct) 1.0 1.0 0.0 null null null)
          (set `self.Dropped` false))))
    (:`then_1`
      (cast `/Game/Blueprints/Character/BP_Body` OtherActor)
      (`PrimitiveComponent.SetSimulatePhysics` (`self.Box`) false))))

(event `CheckColision`
  (bind _location (.location (`self.GetTransform`)))
  ;[0.3953 1 0.2782] Raycasting to check colision
  (bind _outhit (`KismetSystemLibrary.BoxTraceSingleForObjects` (- _location (0.0 0.0 -220.0)) (+ _location (0.0 0.0 0.0)) (110.0 110.0 5.0) (.rotation (`self.GetTransform`)) (`|MakeArray` "ObjectTypeQuery1" :!type "EObjectTypeQuery Enum")))
  (if (`GameplayStatics.BreakHitResult` _outhit)
    (set `self.Overlaped` true)
    (else
      (set `self.Overlaped` false))))

(event `self.ReceiveTick`
  (params (DeltaSeconds :type "Float (single-precision)"))
  ;[0.3953 1 0.2782] Raycasting to check colision
)

(fn `StartPushPull`)

(fn `UserConstructionScript`)