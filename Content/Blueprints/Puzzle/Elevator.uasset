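; Puzzle elevator that rises when all of its linked pressure plates are activated.
; PlateActivated counts active plates, lifting on a full match, otherwise printing the count and reversing the lift.
; Lifting plays a heavy machinery sound and runs the MoveElevator timeline, which lerps the actor upward on Z by FinalPosition from its construction-time location.
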(event `PlateActivated`
  (bind _pressureplates (`self.PressurePlates`))
  (bind _counter (`self.Counter`))
  ;[1 1 1] A plate has been activated, check if door can be opened
  (set `self.Counter` 0)
  (for _array_element _pressureplates
    (if (`/Game/Blueprints/Puzzle/PressurePlate.IsActivated` _array_element)
      (set `self.Counter` (+ (`self.Counter`) 1))))
  (if (== (`KismetArrayLibrary.Array_Length` _pressureplates) _counter)
    (`self.LiftElevator`)
    (else
      (`KismetSystemLibrary.PrintString` (`KismetStringLibrary.Conv_IntToString` _counter))
      (`self.UnliftElevator`))))

(event `LiftElevator`
  (bind _initialposition (`self.InitialPosition`))
  ;[0.3953 1 0.2782] Play up/down animation on elevator triggered
  (`GameplayStatics.PlaySoundAtLocation` "/Game/Sounds/SFX_Elevator_OneShot_TS_Machine_Elevator_Heavy_Door.SFX_Elevator_OneShot_TS_Machine_Elevator_Heavy_Door" (`self.K2_GetActorLocation`) (struct) 1.0 1.0 0.0 null null null)
  (bind (_direction _movement) (`Timeline|MoveElevator` :!label _label)
    (:`Update`
      (`self.K2_SetActorLocation` (`KismetMathLibrary.VLerp` _initialposition (`KismetMathLibrary.MakeVector` (.x _initialposition) (.y _initialposition) (+ (.z _initialposition) (`self.FinalPosition`))) _movement)))))

(event `UnliftElevator`
  ;[0.3953 1 0.2782] Play up/down animation on elevator triggered
  (goto _label :!via `Reverse`))

(fn `UserConstructionScript`
  (set `self.InitialPosition` (`self.K2_GetActorLocation`)))