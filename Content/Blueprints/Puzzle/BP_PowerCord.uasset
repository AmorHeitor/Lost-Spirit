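; Puzzle power cord actor that visually and audibly powers on or off through its activate and deactivate events.
; The construction script builds spline mesh segments along the PowerCord spline and stores them in SMPowerCord.
; Each event plays a sound and a timeline that lerps emissive intensity and an adaptive material parameter on every segment.
; The timeline updates create a dynamic material instance per segment on every tick rather than caching them.
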(event `Acitvated`
  ;[0.3953 1 0.2782] I will kill you if you touch this
  (`GameplayStatics.PlaySoundAtLocation` "/Game/Sounds/PowerCord/S_PowerCordOn.S_PowerCordOn" (`self.K2_GetActorLocation`) (struct) 1.0 1.0 0.0 null null null)
  (bind (_direction _newtrack_0) (`Timeline|Alpha2` :!via `PlayFromStart`)
    (:`Update`
      (for _array_element (`self.SM_PowerCord`)
        (bind _returnvalue (`PrimitiveComponent.CreateDynamicMaterialInstance` _array_element 1 "/Game/Art/Materials/M_MasterMaterials_Inst.M_MasterMaterials_Inst" "None"))
        (`MaterialInstanceDynamic.SetScalarParameterValue` _returnvalue "AdaptiveMaterialFeature" (`KismetMathLibrary.Lerp` 1.0 0.1 _newtrack_0))
        (`MaterialInstanceDynamic.SetScalarParameterValue` _returnvalue "EmissiveIntensity" (`KismetMathLibrary.Lerp` 0.1 100.0 _newtrack_0))))))

(event `Deactivated`
  ;[0.3953 1 0.2782] I will kill you if you touch this
  (`GameplayStatics.PlaySoundAtLocation` "/Game/Sounds/PowerCord/SFX_PowerDownCord_Loop_TS_Power_Down_Air_Light.SFX_PowerDownCord_Loop_TS_Power_Down_Air_Light" (`self.K2_GetActorLocation`) (struct) 1.0 1.0 0.0 null null null)
  (bind (_direction _alpha) (`Timeline|Alpha1` :!via `PlayFromStart`)
    (:`Update`
      (for _array_element (`self.SM_PowerCord`)
        (bind _returnvalue (`PrimitiveComponent.CreateDynamicMaterialInstance` _array_element 1 "/Game/Art/Materials/M_MasterMaterials_Inst.M_MasterMaterials_Inst" "None"))
        (`MaterialInstanceDynamic.SetScalarParameterValue` _returnvalue "AdaptiveMaterialFeature" (`KismetMathLibrary.Lerp` 0.1 1.0 _alpha))
        (`MaterialInstanceDynamic.SetScalarParameterValue` _returnvalue "EmissiveIntensity" (`KismetMathLibrary.Lerp` 150.0 0.1 _alpha))))))

(fn `UserConstructionScript`
  ;[0.3953 1 0.2782] Setting the power cord
  (for _index (range (`SplineComponent.GetNumberOfSplinePoints` (`self.PowerCord`)))
    (bind _returnvalue (`AddComponent|NODE_AddSplineMeshComponent-0`))
    (`KismetArrayLibrary.Array_Add` (`self.SM_PowerCord`) _returnvalue)
    (`SplineMeshComponent.SetForwardAxis` _returnvalue "X" true)
    (bind (_location _tangent) (`SplineComponent.GetLocationAndTangentAtSplinePoint` (`self.PowerCord`) _index "Local"))
    (bind (_location_2 _tangent_2) (`SplineComponent.GetLocationAndTangentAtSplinePoint` (`self.PowerCord`) (+ _index 1) "Local"))
    (`SplineMeshComponent.SetStartAndEnd` _returnvalue _location _tangent _location_2 _tangent_2 true)))