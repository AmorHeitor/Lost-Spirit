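; Puzzle pressure plate that activates a linked door, elevator or final gate when a tagged box, body or either (per PlateType) rests on it.
; Overlap begin lowers or raises the top plate via a timeline with sound, powers the cord and spawns particles.
; End overlap reverses everything once the area is empty; a DoOnce stops Both plates re-triggering.
; The construction script picks square, hexagon or circle meshes by type.
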(event `Particles`
  (`NiagaraFunctionLibrary.SpawnSystemAtLocation` "/Game/Art/Particules/VF_PressurePlate_System.VF_PressurePlate_System" (`self.K2_GetActorLocation`)))

(event `self.DetectionArea.OnComponentBeginOverlap`
  (params (OverlappedComponent :type "PrimitiveComponent Object Reference") (OtherActor :type "Actor Object Reference") (OtherComp :type "PrimitiveComponent Object Reference") (OtherBodyIndex :type Integer) (bFromSweep :type Boolean) (SweepResult :type "HitResult Structure (by ref)"))
  (bind _returnvalue (`self.ActorHasTag` OtherActor "Body"))
  (bind _returnvalue_2 (`self.ActorHasTag` OtherActor "MovableBox"))
  ;[0.3953 1 0.2782] Open door when correct box is on top
  (switch `/Game/Blueprints/Ingredients/Enum_Plataform` (`self.PlateType`)
    (:`NewEnumerator0`
      (if _returnvalue_2
        (set `self.IsActivated` true)
        (`self.PlayAnimation`)
        (switch `/Game/Blueprints/Ingredients/Enum_Triggers` (`self.Trigger`)
          (:`NewEnumerator0`
            (`/Game/Blueprints/Puzzle/InteractableDoor.PlateActivated` (`self.Door`))
            (`/Game/Blueprints/Puzzle/BP_PowerCord.Acitvated` (`self.PowerCord`))
            (`self.Particles`))
          (:`NewEnumerator1`
            (`/Game/Blueprints/Puzzle/Elevator.PlateActivated` (`self.Elevator`))
            (`/Game/Blueprints/Puzzle/BP_PowerCord.Acitvated` (`self.PowerCord`))
            (`self.Particles`))
          (:`NewEnumerator2`
            (`/Game/Blueprints/Puzzle/BP_FinalDoor.PlateActivated` (`self.FinalGate`))
            (`/Game/Blueprints/Puzzle/BP_PowerCord.Acitvated` (`self.PowerCord`))
            (`self.Particles`)))))
    (:`NewEnumerator1`
      (if (or _returnvalue_2 _returnvalue)
        (set `self.ObjectOn` true)
        (set `self.IsActivated` true)
        (`/Engine/EditorBlueprintResources/StandardMacros.DoOnce` false :!label _label
          (:`Completed`
            (`self.PlayAnimation`)
            (switch `/Game/Blueprints/Ingredients/Enum_Triggers` (`self.Trigger`)
              (:`NewEnumerator0`
                (`/Game/Blueprints/Puzzle/InteractableDoor.PlateActivated` (`self.Door`))
                (`/Game/Blueprints/Puzzle/BP_PowerCord.Acitvated` (`self.PowerCord`))
                (`self.Particles`))
              (:`NewEnumerator1`
                (`/Game/Blueprints/Puzzle/Elevator.PlateActivated` (`self.Elevator`))
                (`/Game/Blueprints/Puzzle/BP_PowerCord.Acitvated` (`self.PowerCord`))
                (`self.Particles`))
              (:`NewEnumerator2`
                (`/Game/Blueprints/Puzzle/BP_FinalDoor.PlateActivated` (`self.FinalGate`))
                (`/Game/Blueprints/Puzzle/BP_PowerCord.Acitvated` (`self.PowerCord`))
                (`self.Particles`)))))))
    (:`NewEnumerator2`
      (if _returnvalue
        (set `self.IsActivated` true)
        (`self.PlayAnimation`)
        (switch `/Game/Blueprints/Ingredients/Enum_Triggers` (`self.Trigger`)
          (:`NewEnumerator0`
            (`/Game/Blueprints/Puzzle/InteractableDoor.PlateActivated` (`self.Door`))
            (`/Game/Blueprints/Puzzle/BP_PowerCord.Acitvated` (`self.PowerCord`))
            (`self.Particles`))
          (:`NewEnumerator1`
            (`/Game/Blueprints/Puzzle/Elevator.PlateActivated` (`self.Elevator`))
            (`/Game/Blueprints/Puzzle/BP_PowerCord.Acitvated` (`self.PowerCord`))
            (`self.Particles`))
          (:`NewEnumerator2`
            (`/Game/Blueprints/Puzzle/BP_FinalDoor.PlateActivated` (`self.FinalGate`))
            (`/Game/Blueprints/Puzzle/BP_PowerCord.Acitvated` (`self.PowerCord`))
            (`self.Particles`)))))))

(event `ResetOnce`
  ;[0.3953 1 0.2782] Open door when correct box is on top
  (goto _label :!via `Reset`))

(event `PlayAnimation`
  (`GameplayStatics.PlaySoundAtLocation` "/Game/Sounds/SFX_PressurePlate1_OneShot_TS_Stone_Drag_Rumble.SFX_PressurePlate1_OneShot_TS_Stone_Drag_Rumble" (`self.K2_GetActorLocation`) (struct) 1.0 1.0 0.0 null null null)
  (bind (_direction _activation _location) (`Timeline|Activated` :!label _label_2)
    (:`Update`
      (`SceneComponent.K2_SetRelativeLocation` (`self.TopPlate`) _location false true))))

(event `ReverseAnimation`
  (`GameplayStatics.PlaySoundAtLocation` "/Game/Sounds/SFX_PressurePlateDrop_OneShot_TS_Rock_Door_Close_Debris.SFX_PressurePlateDrop_OneShot_TS_Rock_Door_Close_Debris" (`self.K2_GetActorLocation`) (struct) 1.0 1.0 0.0 null null null)
  (goto _label_2 :!via `Reverse`))

(event `self.DetectionArea.OnComponentEndOverlap`
  (params (OverlappedComponent :type "PrimitiveComponent Object Reference") (OtherActor :type "Actor Object Reference") (OtherComp :type "PrimitiveComponent Object Reference") (OtherBodyIndex :type Integer))
  (bind _returnvalue (`self.ActorHasTag` OtherActor "MovableBox"))
  (bind _returnvalue_2 (`self.ActorHasTag` OtherActor "Body"))
  ;[0.3953 1 0.2782] Close door when box removed from plate
  (if (not (>= (`KismetArrayLibrary.Array_Length` (`PrimitiveComponent.GetOverlappingActors` (`self.DetectionArea`) null)) 1))
    (switch `/Game/Blueprints/Ingredients/Enum_Plataform` (`self.PlateType`)
      (:`NewEnumerator0`
        (if _returnvalue
          (set `self.IsActivated` false)
          (`self.ReverseAnimation`)
          (switch `/Game/Blueprints/Ingredients/Enum_Triggers` (`self.Trigger`)
            (:`NewEnumerator0`
              (`/Game/Blueprints/Puzzle/InteractableDoor.DoorClosed` (`self.Door`))
              (`/Game/Blueprints/Puzzle/BP_PowerCord.Deactivated` (`self.PowerCord`)))
            (:`NewEnumerator1`
              (`/Game/Blueprints/Puzzle/Elevator.UnliftElevator` (`self.Elevator`))
              (`/Game/Blueprints/Puzzle/BP_PowerCord.Deactivated` (`self.PowerCord`)))
            (:`NewEnumerator2`
              (`/Game/Blueprints/Puzzle/BP_FinalDoor.PortalClosed` (`self.FinalGate`))
              (`/Game/Blueprints/Puzzle/BP_PowerCord.Deactivated` (`self.PowerCord`))))))
      (:`NewEnumerator1`
        (if (or _returnvalue _returnvalue_2)
          (set `self.IsActivated` false)
          (`self.ReverseAnimation`)
          (`self.ResetOnce`)
          (switch `/Game/Blueprints/Ingredients/Enum_Triggers` (`self.Trigger`)
            (:`NewEnumerator0`
              (`/Game/Blueprints/Puzzle/InteractableDoor.DoorClosed` (`self.Door`))
              (`/Game/Blueprints/Puzzle/BP_PowerCord.Deactivated` (`self.PowerCord`)))
            (:`NewEnumerator1`
              (`/Game/Blueprints/Puzzle/Elevator.UnliftElevator` (`self.Elevator`))
              (`/Game/Blueprints/Puzzle/BP_PowerCord.Deactivated` (`self.PowerCord`)))
            (:`NewEnumerator2`
              (`/Game/Blueprints/Puzzle/BP_FinalDoor.PortalClosed` (`self.FinalGate`))
              (`/Game/Blueprints/Puzzle/BP_PowerCord.Deactivated` (`self.PowerCord`))))))
      (:`NewEnumerator2`
        (if _returnvalue_2
          (set `self.IsActivated` false)
          (`self.ReverseAnimation`)
          (switch `/Game/Blueprints/Ingredients/Enum_Triggers` (`self.Trigger`)
            (:`NewEnumerator0`
              (`/Game/Blueprints/Puzzle/InteractableDoor.DoorClosed` (`self.Door`))
              (`/Game/Blueprints/Puzzle/BP_PowerCord.Deactivated` (`self.PowerCord`)))
            (:`NewEnumerator1`
              (`/Game/Blueprints/Puzzle/Elevator.UnliftElevator` (`self.Elevator`))
              (`/Game/Blueprints/Puzzle/BP_PowerCord.Deactivated` (`self.PowerCord`)))
            (:`NewEnumerator2`
              (`/Game/Blueprints/Puzzle/BP_FinalDoor.PortalClosed` (`self.FinalGate`))
              (`/Game/Blueprints/Puzzle/BP_PowerCord.Deactivated` (`self.PowerCord`)))))))))

(fn `SetPlate`
  (params (PlateType :type "/Game/Blueprints/Ingredients/Enum_Plataform Enum" :default "NewEnumerator0"))
  ;[0.3953 1 0.2782] Setting new pressure plate
  (set `self.PlateType` PlateType)
  (`StaticMeshComponent.SetStaticMesh` (`self.Plate`) (select `/Game/Blueprints/Ingredients/Enum_Plataform` (`self.PlateType`) :`NewEnumerator0` "/Game/Art/Props/SM_Square_Bottom.SM_Square_Bottom" :`NewEnumerator1` "/Game/Art/Props/SM_Hexagon_Bottom.SM_Hexagon_Bottom" :`NewEnumerator2` "/Game/Art/Props/SM_Circle_Bottom.SM_Circle_Bottom" :!type "StaticMesh Object Reference"))
  (`StaticMeshComponent.SetStaticMesh` (`self.TopPlate`) (select `/Game/Blueprints/Ingredients/Enum_Plataform` (`self.PlateType`) :`NewEnumerator0` "/Game/Art/Props/SM_Square_Top.SM_Square_Top" :`NewEnumerator1` "/Game/Art/Props/SM_Hexagon_Top.SM_Hexagon_Top" :`NewEnumerator2` "/Game/Art/Props/SM_Circle_Top.SM_Circle_Top" :!type "StaticMesh Object Reference")))

(fn `UserConstructionScript`
  ;[0.3953 1 0.2782] Setting new pressure plate
  (`self.SetPlate` (`self.PlateType`)))