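; BP_FinalDoor is a portal door that opens once every linked pressure plate is active.
; Opening and closing toggle collision, FX and sound, with timelines blending a dynamic material; a separate FinalClosed event swaps materials to seal it.
; Its trigger repels the player while closed, or briefly shows the puzzle number once and saves it to the GameInstance.
; A teleport trigger plays one-time ghost camera shake, sound and controller rumble.
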(event `PlateActivated`
  (bind _pressureplates (`self.PressurePlates`))
  ;[1 1 1] A plate has been activated, check if door can be opened
  (set `self.Counter` 0)
  (for _array_element _pressureplates
    (if (`/Game/Blueprints/Puzzle/PressurePlate.IsActivated` _array_element)
      (set `self.Counter` (+ (`self.Counter`) 1))))
  (if (== (`KismetArrayLibrary.Array_Length` _pressureplates) (`self.Counter`))
    (`self.PortalOpen`)))

(event `self.Teleport_Trigger.OnComponentBeginOverlap`
  (params (OverlappedComponent :type "PrimitiveComponent Object Reference") (OtherActor :type "Actor Object Reference") (OtherComp :type "PrimitiveComponent Object Reference") (OtherBodyIndex :type Integer) (bFromSweep :type Boolean) (SweepResult :type "HitResult Structure (by ref)"))
  ;[0.4485 1 0.3441] Plays teleport sound when the player walks through the door
  (`/Engine/EditorBlueprintResources/StandardMacros.DoOnce` false
    (:`Completed`
      (bind _asbp_ghost (cast `/Game/Blueprints/Character/BP_Ghost` OtherActor))
      (`/Game/Blueprints/Character/BP_Ghost.CameraShake` _asbp_ghost)
      (`GameplayStatics.PlaySoundAtLocation` "/Game/Sound/FX/Gate/SFX_PortalTeleport_OneShot_TS_Teleport_06.SFX_PortalTeleport_OneShot_TS_Teleport_06" (`SceneComponent.K2_GetComponentLocation` (`self.Door`)) (struct) 1.0 1.0 0.0 null null null)
      (`PlayerController.ClientPlayForceFeedback` (`GameplayStatics.GetPlayerController` 0) "/Game/Blueprints/Controller/Wall_Feedback.Wall_Feedback" false false "None"))))

(event `PortalOpen`
  (bind _door (`self.Door`))
  ;[0.3953 1 0.2782] Play slide animation on door opened and closed
  (set `self.PortalOpened` true)
  (`PrimitiveComponent.SetCollisionEnabled` _door "NoCollision")
  (`GameplayStatics.PlaySoundAtLocation` "/Game/Sound/FX/Gate/SFX_PortalOpen_OneShot_TS_Time_Portal_Open_Close.SFX_PortalOpen_OneShot_TS_Time_Portal_Open_Close" (`SceneComponent.K2_GetComponentLocation` _door) (struct) 1.0 1.0 0.0 null null null)
  (`ActorComponent.SetActive` (`self.OpenFX`) true false)
  (`ActorComponent.Deactivate` (`self.ClosedFX`))
  (bind (_direction _velocity) (`Timeline|Portal` :!via `PlayFromStart` :!label _label)
    (:`Update`
      (`MaterialInstanceDynamic.SetScalarParameterValue` (stale `self.ReceiveBeginPlay` _returnvalue) "Blend" _velocity))))

(event `PortalClosed`
  (bind _door (`self.Door`))
  ;[0.3953 1 0.2782] Play slide animation on door opened and closed
  (set `self.PortalOpened` false)
  (`PrimitiveComponent.SetCollisionEnabled` _door "QueryAndPhysics")
  (`GameplayStatics.PlaySoundAtLocation` "/Game/Sound/FX/Gate/SFX_PortalClose_OneShot_TS_Time_Portal_Open_Close.SFX_PortalClose_OneShot_TS_Time_Portal_Open_Close" (`SceneComponent.K2_GetComponentLocation` _door) (struct) 1.0 1.0 0.0 null null null)
  (`ActorComponent.Deactivate` (`self.OpenFX`))
  (`ActorComponent.Activate` (`self.ClosedFX`) false)
  (goto _label :!via `Reverse`))

(event `self.Trigger.OnComponentBeginOverlap`
  (params (OverlappedComponent :type "PrimitiveComponent Object Reference") (OtherActor :type "Actor Object Reference") (OtherComp :type "PrimitiveComponent Object Reference") (OtherBodyIndex :type Integer) (bFromSweep :type Boolean) (SweepResult :type "HitResult Structure (by ref)"))
  (if (`self.PortalOpened`)
    ;[1 1 1] Show puzzle number
    (if (and (not (`self.UIShownOnce`)) (!= (`self.PuzzleNumber`) 0))
      (bind _returnvalue (`|CreateWidget` "/Game/UI/Widgets/WI_PuzzleNumber.WI_PuzzleNumber_C"))
      (bind _output_get (set `/Game/UI/Widgets/WI_PuzzleNumber.PuzzleNumber` (`KismetStringLibrary.Concat_StrStr` (`KismetStringLibrary.Conv_IntToString` (`self.PuzzleNumber`)) "/8") _returnvalue))
      (`UserWidget.AddToViewport` _returnvalue 0)
      (`KismetSystemLibrary.Delay` 3.0)
      (`Widget.RemoveFromParent` _returnvalue)
      (set `self.UIShownOnce` true)
      (bind _asbp_game_instance (cast `/Game/Blueprints/Game/BP_GameInstance` (`GameplayStatics.GetGameInstance`)))
      (set `/Game/Blueprints/Game/BP_GameInstance.PuzzleNumber` _output_get _asbp_game_instance))
    (else
      (`NiagaraFunctionLibrary.SpawnSystemAtLocation` "/Game/Art/Particules/FX_NopePortal_System.FX_NopePortal_System" (- (`self.K2_GetActorLocation` OtherActor) (-150.0 0.0 0.0)) (struct :`Pitch` 90.0))
      (`Character.LaunchCharacter` (`GameplayStatics.GetPlayerCharacter` 0) (-2000.0 0.0 0.0) true false))))

(event `self.ReceiveBeginPlay`
  (bind _door (`self.Door`))
  (bind _returnvalue (`PrimitiveComponent.CreateDynamicMaterialInstance` _door 0 (`PrimitiveComponent.GetMaterial` _door 0) "None")))

(event `FinalClosed`
  ;[0.3953 1 0.2782] Setting final closed door
  (bind _returnvalue (`PrimitiveComponent.CreateDynamicMaterialInstance` (`self.Door`) 0 "/Game/Art/Materials/M_FinalDoorDynamic_Inst.M_FinalDoorDynamic_Inst" "None"))
  (bind (_direction _closed) (`Timeline|Closed` :!via `PlayFromStart`)
    (:`Update`
      (`MaterialInstanceDynamic.SetScalarParameterValue` _returnvalue "Blend" _closed)
      (`PrimitiveComponent.SetCollisionEnabled` (`self.Door`) "QueryAndPhysics")
      (`ActorComponent.Deactivate` (`self.OpenFX`)))))

(fn `UserConstructionScript`)