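; MoveableBox is a puzzle box actor that a player can push or pull.
; StartMoving caches a raised Z and runs StartPushPull, which, if the player can move blocks, copies their horizontal velocity onto the box's physics and holds it at that height.
; StopMoving snaps Z to the cached height and clears the adjustment flag.
; A translucent-named material shows while moving, reverting on stop or when trigger overlaps end.
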(event `StartMoving`
  (params (Player :type "/Game/Blueprints/Character/BP_Body Object Reference"))
  (bind (_returnvalue_x _returnvalue_y _returnvalue_z) (`KismetMathLibrary.BreakVector` (`self.K2_GetActorLocation`)))
  ;[0.3953 1 0.2782] Start pushing or pulling box
  (if (not (`self.Adjusted`))
    (set `self.ZForPush` (+ _returnvalue_z 25.0))
    (set `self.Adjusted` true))
  (set `self.Player` Player)
  (`self.StartPushPull`)
  (`PrimitiveComponent.SetMaterial` (`self.Box`) 0 "/Game/Art/Materials/M_MovableBoxTrans.M_MovableBoxTrans"))

(event `self.ReceiveBeginPlay`
  (bind (_returnvalue_x _returnvalue_y _returnvalue_z) (`KismetMathLibrary.BreakVector` (`self.K2_GetActorLocation`)))
  ;[1 1 1] Get box's initial z location
  (set `self.ZForPush` (+ _returnvalue_z 25.0)))

(event `StopMoving`
  (bind (_returnvalue_x _returnvalue_y) (`KismetMathLibrary.BreakVector` (`self.K2_GetActorLocation`)))
  ;[1 1 1] Return box to its original location
  (`self.K2_SetActorLocation` (`KismetMathLibrary.MakeVector` _returnvalue_x _returnvalue_y (`self.ZForPush`)))
  (set `self.ZForPush` (- (`self.ZForPush`) 1.0))
  (`PrimitiveComponent.SetMaterial` (`self.Box`) 0 "/Game/Art/Materials/M_MovableBox.M_MovableBox")
  (set `self.Adjusted` false))

(event `self.Y_Box.OnComponentEndOverlap`
  (params (OverlappedComponent :type "PrimitiveComponent Object Reference") (OtherActor :type "Actor Object Reference") (OtherComp :type "PrimitiveComponent Object Reference") (OtherBodyIndex :type Integer))
  ;[0.3953 1 0.2782] Setting normal material when players leave the area
  (`PrimitiveComponent.SetMaterial` (`self.Box`) 0 "/Game/Art/Materials/M_MovableBox.M_MovableBox"))

(event `self.X_Box.OnComponentEndOverlap`
  (params (OverlappedComponent :type "PrimitiveComponent Object Reference") (OtherActor :type "Actor Object Reference") (OtherComp :type "PrimitiveComponent Object Reference") (OtherBodyIndex :type Integer))
  ;[0.3953 1 0.2782] Setting normal material when players leave the area
  (`PrimitiveComponent.SetMaterial` (`self.Box`) 0 "/Game/Art/Materials/M_MovableBox.M_MovableBox"))

(event `self.Center_Box.OnComponentEndOverlap`
  (params (OverlappedComponent :type "PrimitiveComponent Object Reference") (OtherActor :type "Actor Object Reference") (OtherComp :type "PrimitiveComponent Object Reference") (OtherBodyIndex :type Integer))
  ;[0.3953 1 0.2782] Setting normal material when players leave the area
  (`PrimitiveComponent.SetMaterial` (`self.Box`) 0 "/Game/Art/Materials/M_MovableBox.M_MovableBox"))

(fn `StartPushPull`
  (bind (_returnvalue_x _returnvalue_y) (`KismetMathLibrary.BreakVector` (`self.K2_GetActorLocation`)))
  (bind (_returnvalue_x_2 _returnvalue_y_2) (`KismetMathLibrary.BreakVector` (`self.GetVelocity` (`self.Player`))))
  ;[1 1 1] Give actor's velocity to box to simulate push and pull
  (if (`/Game/Blueprints/Character/BP_Body.CanMoveBlock` (`self.Player`))
    (`PrimitiveComponent.SetPhysicsLinearVelocity` (`self.Box`) (`KismetMathLibrary.MakeVector` _returnvalue_x_2 _returnvalue_y_2) false "None")
    (`self.K2_SetActorLocation` (`KismetMathLibrary.MakeVector` _returnvalue_x _returnvalue_y (`self.ZForPush`)))))

(fn `UserConstructionScript`)