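; Puzzle door that slides open with a rolling-gate sound once every linked pressure plate is activated.
; PlateActivated counts active plates, printing the count until all are active, then DoorOpened plays the SlidingDoor timeline, which offsets the door from its initial position.
; DoorClosed reverses it with sound, while CloseWhenFinished reverses it silently and sets PuzzleFinished.
; The step that would move Collision is disconnected.
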(event `PlateActivated`
  (bind _pressureplates (`self.PressurePlates`))
  (bind _counter (`self.Counter`))
  ;[1 1 1] A plate has been activated, check if door can be opened
  (set `self.Counter` 0)
  (for _array_element _pressureplates
    (if (`/Game/Blueprints/Puzzle/PressurePlate.IsActivated` _array_element)
      (set `self.Counter` (+ (`self.Counter`) 1))))
  (if (== (`KismetArrayLibrary.Array_Length` _pressureplates) _counter)
    (`self.DoorOpened`)
    (else
      (`KismetSystemLibrary.PrintString` (`KismetStringLibrary.Conv_IntToString` _counter)))))

(event `CloseWhenFinished`
  ;[0.3953 1 0.2782] Close door behind the player
  (set `self.PuzzleFinished` true)
  ;[0.3953 1 0.2782] Play slide animation on door opened and closed
  (bind (_direction _doorslide) (`Timeline|SlidingDoor` :!via `Reverse` :!label _label)
    (:`Update`
      (`SceneComponent.K2_SetRelativeLocation` (`self.Door`) (+ _doorslide (`self.IntialPosition`)) false false))))

(event `DoorOpened`
  ;[0.3953 1 0.2782] Play slide animation on door opened and closed
  (`GameplayStatics.PlaySoundAtLocation` "/Game/Sounds/Gates/SFX_GateOpen_OneShot_TS_Door_Rolling_Heavy_ST.SFX_GateOpen_OneShot_TS_Door_Rolling_Heavy_ST" (`self.K2_GetActorLocation`) (struct) 1.0 1.0 0.0 null null null)
  (goto _label))

(event `DoorClosed`
  ;[0.3953 1 0.2782] Play slide animation on door opened and closed
  (`GameplayStatics.PlaySoundAtLocation` "/Game/Sounds/Gates/SFX_GateOpen_OneShot_TS_Door_Rolling_Heavy_ST.SFX_GateOpen_OneShot_TS_Door_Rolling_Heavy_ST" (`self.K2_GetActorLocation`) (struct) 1.0 1.0 0.0 null null null)
  (goto _label :!via `Reverse`))

(event `self.ReceiveBeginPlay`
  ;[0.3953 1 0.2782] Get initial door position
  (set `self.IntialPosition` (`SceneComponent.RelativeLocation` (`self.Door`)))
  (set `self.InitialPositionCol` (`SceneComponent.RelativeLocation` (`self.Collision`))))

(fn `UserConstructionScript`)